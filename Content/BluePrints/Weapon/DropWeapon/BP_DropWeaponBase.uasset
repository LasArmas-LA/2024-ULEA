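; BP_DropWeaponBase is a base weapon pickup that swaps the player's current weapon when interacted with.
; Its OverlapTrigger caches the player pawn on begin overlap and never clears it on end overlap.
; HasInteracted spawns SpawnWeaponClass at the pickup's transform, casts the cached actor to BP_FPS_NFG, destroys its current weapon and equips the new one.
; The pickup does not destroy itself here.
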(event `/Game/BluePrints/Weapon/BPI_Interact.HasInteracted`
  (bind _returnvalue (`|SpawnActorFromClass` (`self.SpawnWeaponClass`) (`self.GetTransform`) "AlwaysSpawn" "MultiplyWithRoot" null null))
  (bind _asbp_fps_nfg (cast `/Game/BluePrints/BP_FPS_NFG` (`self.OverlapActor`)))
  (`self.K2_DestroyActor` (`/Game/BluePrints/BP_FPS_NFG.CurrentWeapon` _asbp_fps_nfg))
  (`/Game/BluePrints/BP_FPS_NFG.EquipWeapon` _asbp_fps_nfg (cast `/Game/BluePrints/Weapon/WeaponMain/BP_WeaponBase` _returnvalue :!pure true)))

(event `self.OverlapTrigger.OnComponentBeginOverlap`
  (params (OverlappedComponent :type "PrimitiveComponent Object Reference") (OtherActor :type "Actor Object Reference") (OtherComp :type "PrimitiveComponent Object Reference") (OtherBodyIndex :type Integer) (bFromSweep :type Boolean) (SweepResult :type "HitResult Structure (by ref)"))
  (if (== OtherActor (`GameplayStatics.GetPlayerPawn` 0))
    (set `self.OverlapActor` OtherActor)))

(event `self.OverlapTrigger.OnComponentEndOverlap`
  (params (OverlappedComponent :type "PrimitiveComponent Object Reference") (OtherActor :type "Actor Object Reference") (OtherComp :type "PrimitiveComponent Object Reference") (OtherBodyIndex :type Integer)))

(fn `UserConstructionScript`)