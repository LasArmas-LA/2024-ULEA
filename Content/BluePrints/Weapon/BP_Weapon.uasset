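; BP_Weapon is a weapon actor that snaps its mesh to a parent's right-hand grip socket and stores a player reference.
; The IA_Switch input toggles full-auto mode through a FlipFlop.
; Disconnected firing logic would start a looping timer, spawn BP_Bullet from the muzzle socket along the camera rotation and play a sound.
; That logic and the timer clear have no triggering event, so neither runs.
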(event `EnhancedInput|/Game/Map/TestWorld/Friends/IA_Switch`
  (params (ActionValue :type Boolean) (ElapsedSeconds :type "Float (double-precision)") (TriggeredSeconds :type "Float (double-precision)") (InputAction :type "InputAction Object Reference" :default "/Game/Map/TestWorld/Friends/IA_Switch.IA_Switch"))
  (:`Started`
    (`/Engine/EditorBlueprintResources/StandardMacros.FlipFlop`
      (:`A`
        (set `self.Is Fullauto` true))
      (:`B`
        (set `self.Is Fullauto` false)))))

(fn `Attach to Hand`
  (params (Parent :type "SceneComponent Object Reference"))
  (`SceneComponent.K2_AttachToComponent` (`self.WeaponMesh`) Parent "GripPoint_r" "SnapToTarget" "SnapToTarget" "KeepWorld" true))

(fn `SetPlayerRef`
  (params (PlayerRef :type "/Game/BluePrints/BP_FPS_NFG Object Reference"))
  (set `self.Player Ref` PlayerRef))

(fn `UserConstructionScript`)