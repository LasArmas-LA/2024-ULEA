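; BP_PistolB is a pistol weapon Blueprint whose Fire event plays the pistol firing animation once and runs a line trace.
; The complex Visibility trace starts at the Barrel socket and is drawn for debugging, with its hit result unused.
; Its end point adds the socket's forward vector times Range to the socket's scale rather than its location.
; BeginPlay and Tick are disabled placeholder nodes.
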(event `/Game/BluePrints/Interface/BPI_Fire.Fire`
  (bind (_returnvalue_location _returnvalue_rotation _returnvalue_scale) (`KismetMathLibrary.BreakTransform` (`self.GetSocketTransform` "Barrel")))
  (`self.PlayAnimation` "/Game/Assets/MilitaryWeapDark/Weapons/Anims/Fire_Pistol_W.Fire_Pistol_W")
  (`KismetSystemLibrary.LineTraceSingle` :`Start` _returnvalue_location :`End` (+ _returnvalue_scale (* (`KismetMathLibrary.GetForwardVector` _returnvalue_rotation) (`self.Range`))) :`TraceChannel` "TraceTypeQuery1" :`bTraceComplex` true :`DrawDebugType` "ForDuration"))