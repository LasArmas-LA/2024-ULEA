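; BP_WeaponBase is a weapon Blueprint that attaches its mesh to a hand and keeps a reference to the player.
; AttachToHand switches on the weapon type enum (AR, SMG, SG, SR, HG) to choose a per-type grip socket on the given parent.
; The mesh snaps to that socket's location and rotation while keeping world scale.
; SetPlayerRef stores the player reference it receives.
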(fn `Attach to Hand`
  (params (Parent :type "SceneComponent Object Reference"))
  ;[0 0 0 1 25] 関数名　Attach To Hand
  ; この関数では列挙型を使用して武器の種類を確認し武器の種類によって持つ位置が変わるように設定されている
  (switch `/Game/BluePrints/Weapon/Enum_WeaponList` (`self.WeaponList`) ; 武器の列挙型
    (:`NewEnumerator0`
      (set `self.Socket Name` "GripPoint_AR"))
    (:`NewEnumerator1`
      (set `self.Socket Name` "GripPoint_SMG"))
    (:`NewEnumerator2`
      (set `self.Socket Name` "GripPoint_SG"))
    (:`NewEnumerator3`
      (set `self.Socket Name` "GripPoint_SR"))
    (:`NewEnumerator4`
      (set `self.Socket Name` "GripPoint_HG")))
  (`SceneComponent.K2_AttachToComponent` (`self.WeaponMesh`) Parent (`self.Socket Name`) "SnapToTarget" "SnapToTarget" "KeepWorld" true) ; 武器を手にアタッチ
)

(fn `SetPlayerRef`
  (params (PlayerRef :type "/Game/BluePrints/BP_FPS_NFG Object Reference"))
  (set `self.Player Ref` PlayerRef))

(fn `UserConstructionScript`)